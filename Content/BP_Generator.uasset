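; BP_Generator is a fuel-fillable generator that shows a WBP_Generator widget while the player character is inside its overlap box.
; The widget is created on BeginPlay, then added to or removed from the viewport on overlap.
; Interaction starts filling when HasFuelCan is true, animating Fuel from 0 to 100 through one of two timelines chosen by FilledOnce.
; The first timeline keeps HasFuelCan true, while the second clears it.
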(event `self.ReceiveBeginPlay`
  (bind _returnvalue (`|CreateWidget` "/Game/WBP_Generator.WBP_Generator_C"))
  (set `self.Gen REF` _returnvalue))

(event `self.Box.OnComponentBeginOverlap`
  (params (OverlappedComponent :type "PrimitiveComponent Object Reference") (OtherActor :type "Actor Object Reference") (OtherComp :type "PrimitiveComponent Object Reference") (OtherBodyIndex :type Integer) (bFromSweep :type Boolean) (SweepResult :type "HitResult Structure (by ref)"))
  (if (== OtherActor (`GameplayStatics.GetPlayerCharacter` 0))
    (`UserWidget.AddToViewport` (`self.Gen REF`) 0)))

(event `self.Box.OnComponentEndOverlap`
  (params (OverlappedComponent :type "PrimitiveComponent Object Reference") (OtherActor :type "Actor Object Reference") (OtherComp :type "PrimitiveComponent Object Reference") (OtherBodyIndex :type Integer))
  (if (== OtherActor (`GameplayStatics.GetPlayerCharacter` 0))
    (bind _gen_ref (`self.Gen REF`)
      (:`then`
        (`Widget.RemoveFromParent` _gen_ref))
      (:`else`))))

(event `/Game/BPI_Interact.interaction`
  (if (`self.Has fuel can?`)
    (`self.fill generator`)))

(event `fill generator`
  (if (not (`self.Filled once`))
    (bind (_direction _newtrack_0) (`Timeline|fill`)
      (:`Update`
        (set `self.Fuel` (`KismetMathLibrary.Lerp` 0.0 100.0 _newtrack_0))
        (set `self.Has fuel can?` true)))
    (else
      (bind (_direction_2 _newtrack_0_2) (`Timeline|Timeline`)
        (:`Update`
          (set `self.Fuel` (`KismetMathLibrary.Lerp` 0.0 100.0 _newtrack_0_2))
          (set `self.Has fuel can?` false))))))

(fn `UserConstructionScript`)