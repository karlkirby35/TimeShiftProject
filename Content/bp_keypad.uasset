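; Interactable keypad actor that opens a linked blocker when the correct code is entered.
; Interaction spawns the WB_KeypadUi widget with a reference back to the keypad, shows the cursor and switches input to UI only.
; The AddDigit event prepends digits to the entered code, while the AddDigitF function appends them.
; The checkcode event compares the entry to the correct code, calling Openblocker on a match or clearing it otherwise.
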(event `/Game/Interaction/BPI_Interact.interaction`
  (bind _returnvalue (`GameplayStatics.GetPlayerController` 0))
  (bind _returnvalue_2 (`|CreateWidget` "/Game/WB_KeypadUi.WB_KeypadUi_C" (`GameplayStatics.GetPlayerController` 0) self))
  (`UserWidget.AddToViewport` _returnvalue_2 0)
  (set `PlayerController.bShowMouseCursor` true _returnvalue)
  (`WidgetBlueprintLibrary.SetInputMode_UIOnlyEx` _returnvalue _returnvalue_2))

(event `AddDigit`
  (params (digit :type String))
  (set `self.enteredcode` (`KismetStringLibrary.Concat_StrStr` digit (`self.enteredcode`)))
  (`KismetSystemLibrary.PrintString` (`self.enteredcode`)))

(event `checkcode`
  (if (`KismetStringLibrary.EqualEqual_StrStr` (`self.correctcode`) (`self.enteredcode`))
    (`/Game/bp_keypadblocker.openblocker` (`self.blockerref`))
    (else
      (`KismetSystemLibrary.PrintString` "wrong code")
      (set `self.enteredcode` ""))))

(fn `addDigitF`
  (params (digit :type String))
  (set `self.enteredcode` (`KismetStringLibrary.Concat_StrStr` (`self.enteredcode`) (`local.digit`))))

(fn `UserConstructionScript`)