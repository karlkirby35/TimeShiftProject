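; Fuel can pickup that the player collects to mark the generator as having fuel.
; On BeginPlay it caches the level's BP_Generator, whose HasFuelCan flag serves as the "hand is full" check.
; Interaction sets that flag, adds a FuelCan entry to the player character's inventory component, reloads the inventory widget and destroys the actor.
; Usefrominventory runs the same check, then sets the flag and destroys the actor without touching the inventory.
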(event `self.ReceiveBeginPlay`
  (bind _returnvalue (`GameplayStatics.GetActorOfClass` "/Game/Interaction/BP_Generator.BP_Generator_C"))
  (set `self.Gen REF` _returnvalue))

(event `/Game/Interaction/BPI_Interact.interaction`
  (if (`/Game/Interaction/BP_Generator.Has fuel can?` (`self.Gen REF`))
    (`KismetSystemLibrary.PrintString` "Hand is full")
    (else
      (set `/Game/Interaction/BP_Generator.Has fuel can?` true (`self.Gen REF`))
      (bind _asbp_first_person_character (cast `/Game/FirstPerson/Blueprints/BP_FirstPersonCharacter` (`GameplayStatics.GetPlayerCharacter` 0)))
      (bind _bp_inventorycomp (`/Game/FirstPerson/Blueprints/BP_FirstPersonCharacter.BP_InventoryComp` _asbp_first_person_character))
      (`KismetArrayLibrary.Array_Add` (`/Game/FirstPerson/Blueprints/BP_InventoryComp.items` _bp_inventorycomp) (make `/Game/Inventory/blueprints/s_itemstructure` "FuelCan" false 2 "/Game/Inventory/models/Screenshot_2026-03-19_163613.Screenshot_2026-03-19_163613"))
      (`/Game/Inventory/widgets/WBP_inventory.loadinventory` (`/Game/FirstPerson/Blueprints/BP_InventoryComp.inventorywidget` _bp_inventorycomp) _bp_inventorycomp)
      (`self.K2_DestroyActor`))))

(fn `usefrominventory`
  (if (`/Game/Interaction/BP_Generator.Has fuel can?` (`self.Gen REF`))
    (`KismetSystemLibrary.PrintString` "Hand is full")
    (else
      (set `/Game/Interaction/BP_Generator.Has fuel can?` true (`self.Gen REF`))
      (`self.K2_DestroyActor`))))

(fn `UserConstructionScript`)