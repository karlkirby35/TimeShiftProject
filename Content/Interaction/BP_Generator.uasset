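; BP_Generator is a fuelable generator that shows a WBP_Generator widget while the player overlaps its box.
; A one-time Interaction searches the player's inventory for a FuelCan and, if found, runs a timeline that raises Fuel and switches the generator on.
; That fill also flags the GL_TimeShift game instance as fueled and, after a delay, updates its objective text.
; An alternate FilledOnce branch animates Fuel with the generator off.
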(event `self.ReceiveBeginPlay`
  (bind _returnvalue (`|CreateWidget` "/Game/WBP_Generator.WBP_Generator_C"))
  (set `self.Gen REF` _returnvalue))

(event `self.Box.OnComponentBeginOverlap`
  (params (OverlappedComponent :type "PrimitiveComponent Object Reference") (OtherActor :type "Actor Object Reference") (OtherComp :type "PrimitiveComponent Object Reference") (OtherBodyIndex :type Integer) (bFromSweep :type Boolean) (SweepResult :type "HitResult Structure (by ref)"))
  (if (== OtherActor (`GameplayStatics.GetPlayerCharacter` 0))
    (`UserWidget.AddToViewport` (`self.Gen REF`) 0)))

(event `self.Box.OnComponentEndOverlap`
  (params (OverlappedComponent :type "PrimitiveComponent Object Reference") (OtherActor :type "Actor Object Reference") (OtherComp :type "PrimitiveComponent Object Reference") (OtherBodyIndex :type Integer))
  (if (== OtherActor (`GameplayStatics.GetPlayerCharacter` 0))
    (bind _gen_ref (`self.Gen REF`)
      (:`then`
        (`Widget.RemoveFromParent` _gen_ref))
      (:`else`))))

(event `/Game/Interaction/BPI_Interact.interaction`
  (`/Engine/EditorBlueprintResources/StandardMacros.DoOnce` false
    (:`Completed`
      (bind _asbp_first_person_character (cast `/Game/FirstPerson/Blueprints/BP_FirstPersonCharacter` (`GameplayStatics.GetPlayerCharacter` 0)))
      (for _array_element (`/Game/FirstPerson/Blueprints/BP_InventoryComp.items` (`/Game/FirstPerson/Blueprints/BP_FirstPersonCharacter.BP_InventoryComp` _asbp_first_person_character))
        (if (`KismetTextLibrary.EqualEqual_TextText` (`.Name_2_6A9E8DDA42F0147B46BF41AC630A7DC1` (break `/Game/Inventory/blueprints/s_itemstructure` _array_element)) "FuelCan")
          (`|ExecutionSequence`
            (:`then_0`
              (break))
            (:`then_1`
              (`self.fill generator`))))))))

(event `fill generator`
  (if (not (`self.Filled once`))
    (bind (_direction _newtrack_0) (`Timeline|fill`)
      (:`Update`
        (set `self.Fuel` (`KismetMathLibrary.Lerp` 0.0 100.0 _newtrack_0))
        (set `self.IsGeneratorOn?` true)
        (bind _asgl_time_shift (cast `/Game/ShiftingManagement/GL_TimeShift` (`GameplayStatics.GetGameInstance`)))
        (set `/Game/ShiftingManagement/GL_TimeShift.generatorfueled` true _asgl_time_shift)
        (bind _asgl_time_shift_2 (cast `/Game/ShiftingManagement/GL_TimeShift` (`GameplayStatics.GetGameInstance`)))
        (`KismetSystemLibrary.Delay` 6.0)
        (set `/Game/ShiftingManagement/GL_TimeShift.currentobj` "Button has been activated somewhere...." _asgl_time_shift_2)))
    (else
      (bind (_direction_2 _newtrack_0_2) (`Timeline|Timeline`)
        (:`Update`
          (set `self.Fuel` (`KismetMathLibrary.Lerp` 0.0 100.0 _newtrack_0_2))
          (set `self.IsGeneratorOn?` false))))))

(fn `UserConstructionScript`)